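; BP_Player is the player pawn, handling movement, mouse look and button-press interaction.
; Axis inputs move it along the capsule's forward and right vectors and drive controller yaw and pitch.
; Interaction calls InteractMessage on the first overlapping actor that implements BP_Interact_Interface.
; A separate SetValues function writes target location, current location as spawn point, and movement type to the pawn's AI controller blackboard.
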(event Input|ActionEvents|InputActionInteraction
  (params (Key :type Key%20Structure :default "None"))
  ;[1 1 1] Button Interaction
  (:Pressed
    (bind _array_element (Utilities|Array|ForEachLoopwithBreak (Collision|GetOverlappingActors 0 :!class /Script/Engine.Actor) :!label _label)
      (:LoopBody
        (if (Utilities|DoesObjectImplementInterface _array_element "/Game/Blueprints/BP_Interact_Interface.BP_Interact_Interface_C")
          (Class|BPInteractInterface|Interact(Message) _array_element)
          (goto _label Break))))))

(event Input|AxisEvents|InputAxisLookUp
  (params (AxisValue :type Float%20%28single-precision%29))
  ;[1 1 1] Mouse Rotation
  (Pawn|Input|AddControllerPitchInput AxisValue))

(event Input|AxisEvents|InputAxisTurn
  (params (AxisValue :type Float%20%28single-precision%29))
  ;[1 1 1] Mouse Rotation
  (Pawn|Input|AddControllerYawInput AxisValue))

(event Input|AxisEvents|InputAxisMoveForward
  (params (AxisValue :type Float%20%28single-precision%29))
  ;[1 1 1] Movement
  (Pawn|Input|AddMovementInput (Math|Vector|GetForwardVector (Variables|Collision|GetCapsuleComponent)) AxisValue false))

(event Input|AxisEvents|InputAxisMoveRight
  (params (AxisValue :type Float%20%28single-precision%29))
  ;[1 1 1] Movement
  (Pawn|Input|AddMovementInput (Math|Vector|GetRightVector (Variables|Collision|GetCapsuleComponent)) AxisValue false))

(fn ConstructionScript)

(fn SetValues
  (params (TargetPoint :type Target%20Point%20Object%20Reference) (MovementType :type E_MovementType%20Enum :default "NewEnumerator0"))
  (bind _self self)
  (bind _returnvalue (AI|GetAIController _self))
  (bind _blackboard (Variables|/Script/AIModule.AIController|GetBlackboard _returnvalue))
  (AI|Components|Blackboard|SetValueasVector _blackboard (Utilities|Name|MakeLiteralName "VTargetPoint") (Transformation|GetActorLocation TargetPoint))
  (AI|Components|Blackboard|SetValueasVector _blackboard (Utilities|Name|MakeLiteralName "VSpawnPoint") (Transformation|GetActorLocation))
  (AI|Components|Blackboard|SetValueasEnum _blackboard (Utilities|Name|MakeLiteralName "MovementType") MovementType))