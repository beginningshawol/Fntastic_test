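; BP_Turtle is an AI-controlled turtle that destroys itself on reaching its assigned target point.
; SetValues stores the target and writes the target location, spawn location and movement type to the AI controller's Blackboard.
; Tick compares turtle and target positions in XY only, within a small tolerance, then calls CommitSudoku.
; CommitSudoku prints a message, plays a game-over sound, spawns a blood splat emitter and destroys the actor.
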(event EventTick
  (params (DeltaSeconds :type Float%20%28single-precision%29))
  (bind _returnvalue (Transformation|GetActorLocation))
  (bind _target_point (Variables|Default|GetTarget%20Point))
  (bind _returnvalue_2 (Transformation|GetActorLocation _target_point))
  (if (Math|Vector|Equal(Vector) (Math|Vector|MakeVector (.x _returnvalue) (.y _returnvalue) 0.0) (Math|Vector|MakeVector (.x _returnvalue_2) (.y _returnvalue_2) 0.0) 1.0)
    (CallFunction|CommitSudoku)))

(fn ConstructionScript)

(fn SetValues
  (params (TargetPoint :type Actor%20Object%20Reference) (MovementType :type E_MovementType%20Enum :default "NewEnumerator0"))
  (bind _self self)
  (bind _returnvalue (AI|GetAIController _self))
  (bind _blackboard (Variables|/Script/AIModule.AIController|GetBlackboard _returnvalue))
  (Variables|Default|SetTarget%20Point TargetPoint)
  (AI|Components|Blackboard|SetValueasVector _blackboard (Utilities|Name|MakeLiteralName "VTargetPoint") (Transformation|GetActorLocation TargetPoint))
  (AI|Components|Blackboard|SetValueasVector _blackboard (Utilities|Name|MakeLiteralName "VSpawnPoint") (Transformation|GetActorLocation))
  (AI|Components|Blackboard|SetValueasEnum _blackboard (Utilities|Name|MakeLiteralName "MovementType") MovementType))

(fn CommitSudoku
  (bind _returnvalue (Transformation|GetActorLocation))
  (Development|PrintString "Commit Sudoku")
  (Audio|PlaySoundatLocation "/Game/Sounds/SC_Discordant_GameOver_Musical_Short.SC_Discordant_GameOver_Musical_Short" _returnvalue "0, 0, 0" 1.0 1.0 0.0 0 0 0)
  (Effects|SpawnEmitteratLocation "/Game/Particles/P_Blood_Splat_Cone.P_Blood_Splat_Cone" _returnvalue)
  (Actor|DestroyActor))